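; Player controller that manages the HUD, enemy targeting, lock-on, interaction and in-game menus for BP_PlayerCharacter.
; Left click camera-traces for a pawn on client and server, then a looping timer refreshes target health and armor on the HUD.
; Tab toggles a timer-driven lock-on that interpolates control yaw toward the target.
; A shorter visibility trace messages interactable Spawn actors, while menu events switch input mode and cursor.
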(event Custom|ShowCharacterMenu
  ;[1 1 1] In Game Character Menu
  (Components|Movement|StopMovementImmediately (Variables|/Script/Engine.Character|GetCharacterMovement (Variables|Default|GetPlayerCharacterRef)))
  (Utilities|IsValid (Variables|Default|GetInteractMenu)
    (:Is%20Valid
      (UserInterface|Viewport|AddtoViewport (Variables|Default|GetInteractMenu) 0))
    (:Is%20Not%20Valid
      (bind _returnvalue (UserInterface|CreateWidget "/Game/Blueprints/Widgets/W_InteractMenu.W_InteractMenu_C" self))
      (Variables|Default|SetInteractMenu _returnvalue)
      (UserInterface|Viewport|AddtoViewport _returnvalue 0)))
  (Input|SetInputModeUIOnly self _returnvalue "DoNotLock")
  (Variables|Default|SetbShowMouseCursor true)
  (Variables|/Game/Blueprints/BP_PlayerCharacter.BP_PlayerCharacter_C|SetStopMovement? (Variables|Default|GetPlayerCharacterRef) true))

(event Custom|LockOnEvent
  ;[1 1 1] Targeting Enemy
  (if (Variables|Default|GetValidTarget?)
    (CallFunction|Lockon (Variables|Default|GetTargetRef))
    (else
      (Default|StopLockonAnimiation (Variables|Default|GetPlayerHud))
      (Utilities|Time|ClearandInvalidateTimerbyHandle (Variables|Default|GetLockOnHandler))
      (Variables|Default|SetLockedOn? false))))

(event Custom|SR_LineTrace
  (params (Controller :type Controller%20Object%20Reference))
  ;[1 0.1042 0.1042] Server
  (bind _asbp_player_character (Utilities|Casting|CastToBP_PlayerCharacter (Pawn|GetControlledPawn Controller)))
  (bind (_outhit _returnvalue) (Collision|LineTraceForObjects (Transformation|GetWorldLocation (Variables|/Game/Blueprints/BP_PlayerCharacter.BP_PlayerCharacter_C|GetCamera _asbp_player_character)) (+ (Transformation|GetWorldLocation (Variables|/Game/Blueprints/BP_PlayerCharacter.BP_PlayerCharacter_C|GetCamera _asbp_player_character)) (* (Math|Vector|GetForwardVector (Variables|/Game/Blueprints/BP_PlayerCharacter.BP_PlayerCharacter_C|GetCamera _asbp_player_character)) 8e+03)) (Variables|Default|GetPawnObject) false (Utilities|Array|MakeArray _asbp_player_character) "None"))
  (if _returnvalue
    (bind _asbp_player_character_2 (Utilities|Casting|CastToBP_PlayerCharacter (.HitActor (Collision|BreakHitResult _outhit))))
    (Variables|Default|SetTargetRef _asbp_player_character_2)
    (else
      (Variables|Default|SetTargetRef 0))))

(event Custom|SetPlayerStatus
  (params (Icon :type Texture%202D%20Object%20Reference))
  ;[1 1 1] Set Status and Debuffs
  (Default|SetStatus (Variables|Default|GetPlayerHud) Icon))

(event Custom|RemovePlayerStatus
  ;[1 1 1] Set Status and Debuffs
  (Default|RemoveStatus (Variables|Default|GetPlayerHud)))

(event Custom|SetActionText
  (params (DisplayText :type Text))
  ;[1 1 1] Action text
  (Default|ActivateActionText (Variables|Default|GetPlayerHud) DisplayText))

(event Custom|UpdateAttributes
  ;[1 1 1] Targeting Enemy
  (CallFunction|SetTargetAttributes))

(event EventBeginPlay
  ;[1 1 1] Initialize
  (bind _returnvalue (UserInterface|CreateWidget "/Game/Blueprints/Widgets/W_PlayerHUD.W_PlayerHUD_C" self))
  (Variables|Default|SetPlayerHud _returnvalue)
  (UserInterface|Viewport|AddtoViewport _returnvalue 0)
  (Input|SetInputModeGameOnly)
  (bind _asbp_player_character (Utilities|Casting|CastToBP_PlayerCharacter (Game|Player|GetPlayerPawn 0)))
  (Variables|Default|SetPlayerCharacterRef _asbp_player_character)
  (Networking|SwitchHasAuthority
    (:Remote
      (CallFunction|ClearTarget))))

(event Input|ActionEvents|InputActionInteract
  (params (Key :type Key%20Structure))
  ;[1 1 1] Interact
  (:Pressed
    (CallFunction|LineTraceInteract)))

(event Input|ActionEvents|InputActionGameMenu
  (params (Key :type Key%20Structure))
  ;[1 1 1] Game Menu
  (:Pressed
    (Utilities|FlowControl|FlipFlop
      (:A
        (bind _returnvalue (UserInterface|CreateWidget "/Game/Blueprints/Widgets/W_GameMenu.W_GameMenu_C" self))
        (Variables|Default|SetGameMenu _returnvalue)
        (UserInterface|Viewport|AddtoViewport _returnvalue 4)
        (Input|SetInputModeGameandUI self _returnvalue "DoNotLock" true)
        (Variables|Default|SetbShowMouseCursor true))
      (:B
        (Widget|RemovefromParent (Variables|Default|GetGameMenu))
        (Input|SetInputModeGameOnly self)
        (Variables|Default|SetbShowMouseCursor false)))))

(event Input|MouseEvents|LeftMouseButton
  (params (Key :type Key%20Structure))
  ;[1 1 1] Targeting Enemy
  (:Pressed
    (CallFunction|SRLineTrace self)
    (bind _validtarget_ (CallFunction|LineTrace))
    (if _validtarget_
      (CallFunction|SetTarget)
      (bind _returnvalue (Utilities|Time|SetTimerbyEvent (delegate Custom|UpdateAttributes) 0.1 true))
      (Variables|Default|SetTargetHandler _returnvalue)
      (else
        (CallFunction|ClearTarget)
        (Utilities|Time|ClearandInvalidateTimerbyHandle (Variables|Default|GetTargetHandler))))))

(event Input|KeyboardEvents|Tab
  (params (Key :type Key%20Structure))
  (bind _playerhud (Variables|Default|GetPlayerHud))
  ;[1 1 1] Targeting Enemy
  (:Pressed
    (if (Variables|Default|GetLockedOn?)
      (Default|StopLockonAnimiation _playerhud :!label _label)
      (Utilities|Time|ClearandInvalidateTimerbyHandle (Variables|Default|GetLockOnHandler))
      (Variables|Default|SetLockedOn? false)
      (elif (Variables|Default|GetValidTarget?)
        (bind _returnvalue (Utilities|Time|SetTimerbyEvent (delegate Custom|LockOnEvent) 0.01 true))
        (Variables|Default|SetLockOnHandler _returnvalue)
        (Utilities|IsValid (Variables|Default|GetTargetRef)
          (:Is%20Valid
            (Default|LockonAnimation _playerhud)
            (Variables|Default|SetLockedOn? true))
          (:Is%20Not%20Valid
            (goto _label)))))))

(fn ConstructionScript)

(fn LineTrace
  (bind _playercharacterref (Variables|Default|GetPlayerCharacterRef))
  (bind _camera (Variables|/Game/Blueprints/BP_PlayerCharacter.BP_PlayerCharacter_C|GetCamera _playercharacterref))
  (bind _returnvalue (Transformation|GetWorldLocation _camera))
  (bind (_outhit _returnvalue_2) (Collision|LineTraceForObjects _returnvalue (+ _returnvalue (* (Math|Vector|GetForwardVector _camera) 8e+03)) (Variables|Default|GetPawnObject) false (Utilities|Array|MakeArray _playercharacterref) "None"))
  (if _returnvalue_2
    (bind _asmy_character (Utilities|Casting|CastToMyCharacter (.HitActor (Collision|BreakHitResult _outhit)))
      (:then
        (Variables|Default|SetTargetRef _asmy_character)
        (bind _output_get (Variables|Default|SetValidTarget? true)))
      (:CastFailed
        (Variables|Default|SetTargetRef 0 :!label _label)
        (Variables|Default|SetValidTarget? false)))
    (else
      (goto _label)))
  (return _output_get))

(fn SetTargetAttributes
  (bind _targetref (Variables|Default|GetTargetRef))
  (bind _playerhud (Variables|Default|GetPlayerHud))
  (Class|IInterface|SetTargetHp(Message) _playerhud (Class|MyCharacter|GetHealthPercent _targetref))
  (Class|IInterface|SetTargetArmor(Message) _playerhud (Class|MyCharacter|GetArmorPercent _targetref)))

(fn ClearTarget
  (bind _playerhud (Variables|Default|GetPlayerHud))
  (Rendering|Components|TextRender|SetText (Variables|/Game/Blueprints/Widgets/W_PlayerHUD.W_PlayerHUD_C|GetTextBlock_TargetName _playerhud) "")
  (Widget|SetRenderOpacity (Variables|/Game/Blueprints/Widgets/W_PlayerHUD.W_PlayerHUD_C|GetProgressBar_TargetHealth _playerhud) 0.0)
  (Widget|SetRenderOpacity (Variables|/Game/Blueprints/Widgets/W_PlayerHUD.W_PlayerHUD_C|GetProgressBar_TargetArmor _playerhud) 0.0))

(fn LineTraceInteract
  (bind _playercharacterref (Variables|Default|GetPlayerCharacterRef))
  (bind _camera (Variables|/Game/Blueprints/BP_PlayerCharacter.BP_PlayerCharacter_C|GetCamera _playercharacterref))
  (bind _returnvalue (Transformation|GetWorldLocation _camera))
  (bind (_outhit _returnvalue_2) (Collision|LineTraceByChannel _returnvalue (+ _returnvalue (* (Math|Vector|GetForwardVector _camera) 8e+02)) "TraceTypeQuery1" false (Utilities|Array|MakeArray _playercharacterref) "None"))
  (if _returnvalue_2
    (bind _asspawn (Utilities|Casting|CastToSpawn (.HitActor (Collision|BreakHitResult _outhit))))
    (Class|IInterface|Interact(Message) _asspawn self)))

(fn Lockon
  (params (Target :type Actor%20Object%20Reference))
  (bind _playercharacterref (Variables|Default|GetPlayerCharacterRef))
  (bind _returnvalue (Pawn|GetController _playercharacterref))
  (bind _returnvalue_2 (Pawn|GetControlRotation _returnvalue :!class /Script/Engine.Controller))
  (bind (_roll _pitch) (Math|Rotator|BreakRotator _returnvalue_2))
  ;[0 0 0] Set Control Rotation
  (Pawn|SetControlRotation (Pawn|GetController (Variables|Default|GetPlayerCharacterRef)) (Math|Rotator|MakeRotator _roll _pitch (.Yaw (Math|Rotator|BreakRotator (Math|Interpolation|RInterpTo _returnvalue_2 (Math|Rotator|FindLookatRotation (Transformation|GetActorLocation (Variables|Default|GetPlayerCharacterRef)) (Transformation|GetActorLocation Target)) (Utilities|Time|GetWorldDeltaSeconds) (Variables|Default|GetInterpolationSpeed)))))))

(fn SetTarget
  (bind _playerhud (Variables|Default|GetPlayerHud))
  (Widget|SetRenderOpacity (Variables|/Game/Blueprints/Widgets/W_PlayerHUD.W_PlayerHUD_C|GetProgressBar_TargetHealth _playerhud) 1.0)
  (bind _asbp_player_character (Utilities|Casting|CastToBP_PlayerCharacter (Variables|Default|GetTargetRef)))
  (Rendering|Components|TextRender|SetText (Variables|/Game/Blueprints/Widgets/W_PlayerHUD.W_PlayerHUD_C|GetTextBlock_TargetName _playerhud) (Variables|/Game/Blueprints/BP_PlayerCharacter.BP_PlayerCharacter_C|GetPlayerName _asbp_player_character)))