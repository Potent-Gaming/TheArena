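; Gameplay Ability for the player's three-hit melee combo against the controller's current target, if within range.
; PlayMontage picks each attack montage by class index and combo counter.
; WaitCombo chains hits on input timed against montage length, otherwise ending the ability using attack-speed delays.
; Completed montages commit cost and apply GE_ComboAbility, passing base damage times a rising per-hit multiplier through SetByCaller.
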(event Ability|EventActivateAbility
  (Utilities|GetActors)
  (Utilities|IsValid (Variables|Default|GetTargetRef)
    (:Is%20Valid
      (Utilities|CheckMeleeRange
        (:true
          (Utilities|PlayMontage
            (:Output
              (Utilities|WaitCombo
                (:true
                  (Utilities|PlayMontage
                    (:Output
                      (Utilities|WaitCombo
                        (:true
                          (Utilities|PlayMontage
                            (:On%20Completed
                              (Utilities|ApplyDamage 1.3 (Variables|Default|GetTargetRef))
                              (Ability|CommitAbilityCost false)
                              (Ability|EndAbility))))))
                    (:On%20Completed
                      (Utilities|ApplyDamage 1.2 (Variables|Default|GetTargetRef))
                      (Ability|CommitAbilityCost false))))))
            (:On%20Completed
              (Utilities|ApplyDamage 1.1 (Variables|Default|GetTargetRef))
              (Ability|CommitAbilityCost false))))
        (:false
          (Ability|EndAbility :!label _label))))
    (:Is%20Not%20Valid
      (goto _label))))

(event Ability|EventOnEndAbility
  (params (bWasCancelled :type Boolean)))

(fn CheckInputPressed
  (if (not (Variables|Default|GetInputPressed?))
    (Ability|EndAbility)))