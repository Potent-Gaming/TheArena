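; GA_Stun is a gameplay ability that applies a five-second stun status to the owning player character.
; It caches the player and controller target, commits, plays a class-based montage, calls SRStun on the player, then ends after the delay.
; Warrior and Berserker montages are rate-scaled to the stun time, while the third class reuses the Warrior montage at default rate.
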(event Ability|EventActivateAbility
  (Variables|Default|SetStunTime 5.0)
  (Utilities|GetActors)
  (Ability|CommitAbility)
  (Utilities|PlayMontage (Variables|Default|GetStunTime))
  (Default|SRStun (Variables|Default|GetOwningPlayer) (Variables|Default|GetStunTime))
  (Ability|Tasks|WaitDelay (Variables|Default|GetStunTime)
    (:OnFinish
      (Ability|EndAbility))))

(event Ability|EventOnEndAbility
  (params (bWasCancelled :type Boolean)))