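; Gameplay ability that roots the player character it runs on for a fixed duration, then grants root immunity.
; On activation it commits, calls Rooted on the player with the root time and a doubled immunity duration, waits out the root, then ends.
; Ending the ability calls Unroot and applies the GE_RootImmune effect to the owner.
; Non-player avatars end the ability immediately.
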(event Ability|EventActivateAbility
  (bind _asbp_player_character (Utilities|Casting|CastToBP_PlayerCharacter (Ability|GetAvatarActorfromActorInfo))
    (:then
      (Variables|Default|SetOwningPlayer _asbp_player_character)
      (Ability|CommitAbility)
      (bind _output_get (Variables|Default|SetRootDuration 15.0))
      (Default|Rooted (Variables|Default|GetOwningPlayer) _output_get (* _output_get 2.0))
      (Utilities|FlowControl|Delay _output_get)
      (Ability|EndAbility))
    (:CastFailed
      (Ability|EndAbility))))

(event Ability|EventOnEndAbility
  (params (bWasCancelled :type Boolean))
  (Default|Unroot (Variables|Default|GetOwningPlayer))
  (Ability|ApplyGameplayEffectToOwner "/Game/Blueprints/Characters/Abilities/Immunities/GE_RootImmune.GE_RootImmune_C"))