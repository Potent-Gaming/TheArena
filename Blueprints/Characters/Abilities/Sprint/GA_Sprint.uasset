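; Sprint gameplay ability that speeds up the player character and shows a status icon while active.
; On activation it commits, multiplies movement speed via SRChangeMovementSpeed and applies the GE_SprintCost effect.
; It ends when input is released or an attribute threshold check matches.
; Ending removes effects tagged Status.Sprinting, divides the speed back and clears the status from player controller 0.
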(event Ability|EventActivateAbility
  (bind _asbp_player_character (Utilities|Casting|CastToBP_PlayerCharacter (Ability|GetAvatarActorfromActorInfo))
    (:then
      (bind _asbp_player_controller (Utilities|Casting|CastToBP_PlayerController (Game|GetPlayerController 0))
        (:then
          (Default|SetPlayerStatus _asbp_player_controller (Variables|Default|GetIcon))
          (Ability|CommitAbility)
          (Default|SRChangeMovementSpeed _asbp_player_character 1.25 "Multiply")
          (Ability|ApplyGameplayEffectToOwner "/Game/Blueprints/Characters/Abilities/Sprint/GE_SprintCost.GE_SprintCost_C")
          (bind _bmatchescomparison (Ability|Tasks|WaitForAttributeChangeThreshold "(AttributeName=\"Endurance\",Attribute=/Script/IntoTheArena.MyAttributeSet:Endurance,AttributeOwner=None)" "LessThanOrEqualTo" 0.0 true 0)
            (:then
              (Ability|Tasks|WaitInputRelease false
                (:OnRelease
                  (bind _output_get (Variables|Default|SetReleasedInput true)))))
            (:OnChange
              _))
          (if (or _output_get _bmatchescomparison)
            (Ability|EndAbility)))
        (:CastFailed
          (Development|PrintString "Cast Failed" :!label _label)
          (Ability|EndAbility))))
    (:CastFailed
      (goto _label))))

(event Ability|EventOnEndAbility
  (params (bWasCancelled :type Boolean))
  (Ability|RemoveGameplayEffectFromOwnerWithAssetTags "(GameplayTags=((TagName=\"Status.Sprinting\")))")
  (bind _asbp_player_character (Utilities|Casting|CastToBP_PlayerCharacter (Ability|GetAvatarActorfromActorInfo)))
  (Default|SRChangeMovementSpeed _asbp_player_character 1.25 "Divide")
  (bind _asbp_player_controller (Utilities|Casting|CastToBP_PlayerController (Game|GetPlayerController 0)))
  (Default|RemovePlayerStatus _asbp_player_controller)
  (Variables|Default|SetReleasedInput false))