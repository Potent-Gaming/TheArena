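; Game mode Blueprint that handles finding, joining and creating online multiplayer sessions for the game world.
; FindWorldSession searches for internet sessions and passes the first result to JoinWorldSession, with no fallback when none is found.
; CreateWorldSession runs only with authority, creates a small non-LAN session, then opens the World level as a listen server and sets game-only input.
; PostLogin is an empty stub.
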(event Custom|CreateWorldSession
  ;[1 1 1] Join or Create Game
  (Networking|SwitchHasAuthority
    (:Authority
      (|Session (Game|GetPlayerController 0) 4 false
        (:OnSuccess
          (Game|OpenLevel(byName) "World" true "Listen")
          (Input|SetInputModeGameOnly (Game|GetPlayerController 0)))))))

(event Custom|FindWorldSession
  ;[1 1 1] Join or Create Game
  (bind _results (|FindSessions (Game|GetPlayerController 0) 0 false)
    (:OnSuccess
      (if (Utilities|Array|IsValidIndex _results)
        (CallFunction|JoinWorldSession (Utilities|Array|Get(acopy) _results))))))

(event Custom|JoinWorldSession
  (params (Session :type Blueprint%20Session%20Result%20Structure))
  ;[1 1 1] Join or Create Game
  (|JoinSession (Game|GetPlayerController 0) Session))

(event EventPostLogin
  (params (NewPlayer :type Player%20Controller%20Object%20Reference)))

(fn ConstructionScript)